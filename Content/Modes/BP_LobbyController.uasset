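; BP_LobbyController is the lobby player controller that manages the lobby menu widget for its player.
; Shortly after BeginPlay it triggers UINeedsUpdate, which creates the menu if missing, adds it to the viewport and refreshes its player list.
; The same event serves to reflect player logins and logouts, while RemoveUI takes the menu off screen.
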(event `UINeedsUpdate`
  ;[1 1 1] Update UI To reflect player login / logout
  (`self.SpawnUIIfNeeded`)
  (`/Game/UI/LobbyMenu.UpdatePlayerList` (`self.LobbyMenu`)))

(event `self.ReceiveBeginPlay`
  ;[1 1 1] Spawn UI
  (`KismetSystemLibrary.Delay` 1.0)
  (`self.UINeedsUpdate`))

(event `RemoveUI`
  (bind _lobbymenu (`self.LobbyMenu`))
  ;[1 1 1] Remove UI
  (`/Engine/EditorBlueprintResources/StandardMacros.IsValid` _lobbymenu
    (:`Is Valid`
      (`Widget.RemoveFromParent` _lobbymenu))))

(fn `UserConstructionScript`)