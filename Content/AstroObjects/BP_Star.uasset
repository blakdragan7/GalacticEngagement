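; BP_Star is a star actor that gives each instance a random size and look through a sprite component.
; Its construction script sets a random uniform scale, then creates a dynamic material on StarSprite with a color picked from StarColors and a random emissive power.
; The randomization is unseeded, so the look rerolls whenever construction reruns, and the event graph has no runtime logic.
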(fn `UserConstructionScript`
  (bind _starcolors (`self.StarColors`))
  (`self.SetActorScale3D` (`KismetMathLibrary.Conv_DoubleToVector` (`KismetMathLibrary.RandomFloatInRange` (`self.StarMinSize`) (`self.StarMaxSize`))))
  (bind _returnvalue (`PrimitiveComponent.CreateDynamicMaterialInstance` (`self.StarSprite`) 0 "/Game/AstroObjects/StarMaterial.StarMaterial"))
  (bind _output_get (set `self.DM_Star` _returnvalue))
  (`MaterialInstanceDynamic.SetVectorParameterValue` _output_get "Color" (`|GetArrayItem` _starcolors (`KismetMathLibrary.RandomInteger` (`KismetArrayLibrary.Array_Length` _starcolors))))
  (`MaterialInstanceDynamic.SetScalarParameterValue` _output_get "EmmisivePower" (`KismetMathLibrary.RandomFloatInRange` (`self.EmmisiveMin`) (`self.EmmisiveMax`))))