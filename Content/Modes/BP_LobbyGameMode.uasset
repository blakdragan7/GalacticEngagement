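; Lobby game mode that tracks connected player controllers and keeps their lobby UI in sync.
; PostLogin adds the new controller to AllControllers and OnLogout removes it, then each tells every BP_LobbyController that its UI needs updating.
; RemoveAllUI loops over the same array to have every lobby controller remove its UI.
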(event `Remove All UI`
  ;[1 1 1] Server Remove All UI
  (for _array_element (`self.AllControllers`)
    (bind _asbp_lobby_controller (cast `/Game/Modes/BP_LobbyController` _array_element))
    (`/Game/Modes/BP_LobbyController.RemoveUI` _asbp_lobby_controller)))

(event `self.K2_PostLogin`
  (params (NewPlayer :type "PlayerController Object Reference"))
  (bind _allcontrollers (`self.AllControllers`))
  ;[1 1 1] Add New Client and Update UI
  (`KismetArrayLibrary.Array_AddUnique` _allcontrollers NewPlayer)
  (for _array_element _allcontrollers
    (bind _asbp_lobby_controller (cast `/Game/Modes/BP_LobbyController` _array_element))
    (`/Game/Modes/BP_LobbyController.UINeedsUpdate` _asbp_lobby_controller)))

(event `self.K2_OnLogout`
  (params (ExitingController :type "Controller Object Reference"))
  (bind _allcontrollers (`self.AllControllers`))
  ;[1 1 1] Remove client and update UI
  (`KismetArrayLibrary.Array_RemoveItem` _allcontrollers ExitingController)
  (for _array_element _allcontrollers
    (bind _asbp_lobby_controller (cast `/Game/Modes/BP_LobbyController` _array_element))
    (`/Game/Modes/BP_LobbyController.UINeedsUpdate` _asbp_lobby_controller)))

(fn `UserConstructionScript`)