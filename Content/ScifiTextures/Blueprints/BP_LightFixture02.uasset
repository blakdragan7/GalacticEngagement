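; BP_LightFixture02 is a configurable spotlight fixture prop with a visible beam volume and dust particles.
; All logic runs in the construction script, applying exposed settings for cone, offset, colour, intensity, attenuation and beam scale and visibility.
; Dynamic material instances tint the beam and dust and set their opacity.
; The light colour also drives the fixture's emissive, multiplied by a clamped glow scale.
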(fn `UserConstructionScript`
  (bind _spotlight (`self.SpotLight`))
  (bind _spotlight_2 (`self.SpotLight`))
  (bind _light_volume (`self.Light volume`))
  (`|ExecutionSequence`
    (:`then_0`
      ;[1 1 1] change light volume size
      (`SceneComponent.SetWorldScale3D` (`self.Light volume`) (`self.Light Volume Size`)))
    (:`then_1`
      ;[1 1 1] particle colour and opacity
      (bind _returnvalue (`PrimitiveComponent.CreateDynamicMaterialInstance` (`self.Dust Particles`) 0 null))
      (`MaterialInstanceDynamic.SetVectorParameterValue` _returnvalue "Particle Color" (`self.Particle Color`)))
    (:`then_2`
      ;[1 1 1] Cone size and offset
      (`SpotLightComponent.SetInnerConeAngle` _spotlight (`self.LightInnerConeX`))
      (`SceneComponent.K2_SetWorldLocation` _spotlight (+ (`SceneComponent.K2_GetComponentLocation` _spotlight) (`self.SpotLightOffset`)) false false)
      ;[1 1 1] Light colour
      (`LightComponent.SetLightColor` (`self.SpotLight`) (`self.LightColor`) true)
      ;[1 1 1] Emissive colour
      (bind _returnvalue_2 (`PrimitiveComponent.CreateDynamicMaterialInstance` (`self.LightFixture`) 0 null))
      (`MaterialInstanceDynamic.SetVectorParameterValue` _returnvalue_2 "Emissive Color" (* (`self.LightColor`) (`KismetMathLibrary.FClamp` (* (`self.GlowScale`) 250.0) 2.0 20.0)))
      ;[1 1 1] Light attenuation and intensity
      (`PointLightComponent.SetAttenuationRadius` _spotlight_2 (`self.LightAttenuation`))
      (`LightComponent.SetIntensity` _spotlight_2 (`self.LightIntensity`))
      ;[1 1 1] Beam opacity and toggle off and on
      (`SpotLightComponent.SetOuterConeAngle` _spotlight_2 (`self.LightOuterConeX`))
      (`SceneComponent.SetVisibility` _light_volume (`self.BeamVisible`) false)
      (bind _returnvalue_3 (`PrimitiveComponent.CreateDynamicMaterialInstance` _light_volume 0 null))
      (`MaterialInstanceDynamic.SetVectorParameterValue` _returnvalue_3 "Color" (`self.LightColor`))
      (`MaterialInstanceDynamic.SetScalarParameterValue` _returnvalue_3 "Opacity" (`self.BeamOpacity`)))
    (:`then_3`
      (bind _returnvalue_4 (`PrimitiveComponent.CreateDynamicMaterialInstance` (`self.Dust Particles`) 0 null))
      (`MaterialInstanceDynamic.SetVectorParameterValue` _returnvalue_4 "Particle Opacity" (`self.ParticleOpacity`)))))