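; Destructible asteroid that drifts at a fixed height and shatters under player projectile fire.
; Construction picks a random mesh and, by a separate roll, a mass; BeginPlay adds random linear and angular impulses, and Tick pins the starting Z.
; GEAmmoBase hits apply radius damage with effects; fracture triggers radial force, dust and explosion sound, then destroys the actor after a delay.
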(event `self.ReceiveBeginPlay`
  (bind _destructible (`self.Destructible`))
  (bind _returnvalue (`KismetMathLibrary.MakeVector` (`KismetMathLibrary.RandomFloatInRange` 0.1 3.0)))
  ;[1 1 1] Give some initial impulse to the spawned asteroid
  (set `self.StartingZ` (.z (`self.K2_GetActorLocation`)))
  (`KismetSystemLibrary.Delay` 0.1)
  (`PrimitiveComponent.AddImpulse` _destructible _returnvalue "None" true)
  (`PrimitiveComponent.AddAngularImpulse` _destructible _returnvalue "None" true))

(event `self.ReceiveHit`
  (params (MyComp :type "PrimitiveComponent Object Reference") (Other :type "Actor Object Reference") (OtherComp :type "PrimitiveComponent Object Reference") (bSelfMoved :type Boolean) (HitLocation :type "Vector Structure") (HitNormal :type "Vector Structure") (NormalImpulse :type "Vector Structure") (Hit :type "HitResult Structure (by ref)"))
  ;[1 1 1] If the asteroids got hit with our projectile, apply damage and play hit effects
  (cast `GEAmmoBase` Other)
  (`DestructibleComponent.ApplyRadiusDamage` (`self.Destructible`) 100.0 HitLocation 1000.0 10000.0 true)
  (`PrimitiveComponent.SetLinearDamping` (`self.Destructible`) 3.0)
  (`GameplayStatics.PlaySoundAtLocation` "/Game/AsteroidsFromPhotogrammetry/Sounds/Wavs/A_Hit.A_Hit")
  (bind _returnvalue (`GameplayStatics.SpawnEmitterAtLocation` "/Game/AsteroidsFromPhotogrammetry/Effects/P_Asteroid_Hit.P_Asteroid_Hit" HitLocation))
  (`SceneComponent.SetRelativeScale3D` _returnvalue (10.0 10.0 10.0)))

(event `destroySelf`
  ;[1 1 1] Destroy the actor of the blasted asteroid
  (`self.K2_DestroyActor`))

(event `self.Destructible.OnComponentFracture`
  (params (HitPoint :type "Vector Structure (by ref)") (HitDirection :type "Vector Structure (by ref)"))
  (bind _destructible (`self.Destructible`))
  (bind _returnvalue (`SceneComponent.K2_GetComponentLocation` _destructible))
  ;[1 1 1] The asteroid got blasted. Apply effects, update score and check if we should spawn a Power Up
  (`KismetSystemLibrary.K2_SetTimer` null "destroySelf" 4.0)
  (`PrimitiveComponent.SetLinearDamping` (`self.Destructible`) 1.8)
  (`PrimitiveComponent.AddRadialForce` _destructible _returnvalue 3000.0 1000000.0 "RIF_Constant" true)
  (bind _returnvalue_2 (`GameplayStatics.SpawnEmitterAtLocation` "/Game/AsteroidsFromPhotogrammetry/Effects/P_Asteroid_Dust_1.P_Asteroid_Dust_1" HitPoint))
  (`SceneComponent.SetRelativeScale3D` _returnvalue_2 (100.0 100.0 100.0))
  (`GameplayStatics.PlaySoundAtLocation` "/Game/AsteroidsFromPhotogrammetry/Sounds/Cues/A_Explosions_Cue.A_Explosions_Cue" HitPoint)
  (bind _returnvalue_3 (`GameplayStatics.SpawnEmitterAtLocation` "/Game/AsteroidsFromPhotogrammetry/Effects/P_Asteroid_Dust_2.P_Asteroid_Dust_2" _returnvalue))
  (`SceneComponent.SetRelativeScale3D` _returnvalue_3 (10.0 10.0 10.0)))

(event `self.ReceiveTick`
  (params (DeltaSeconds :type "Float (single-precision)"))
  ;[1 1 1] Force Z Location
  (`self.K2_SetActorLocation` (`KismetMathLibrary.MakeVector` (.x (`self.K2_GetActorLocation`)) (.y (`self.K2_GetActorLocation`)) (`self.StartingZ`))))

(fn `UserConstructionScript`
  (locals (Asteroids :type "Array of DestructibleMesh Object Reference"))
  (bind _returnvalue (`KismetMathLibrary.RandomIntegerInRange` 0 8))
  (bind _destructible (`self.Destructible`))
  ;[1 1 1] Select a random asteroid mesh (to spawn) and set it's mass for the physics simulation
  (`DestructibleComponent.SetDestructibleMesh` _destructible (`|GetArrayItem` (`local.Asteroids`) _returnvalue))
  (switch `int` _returnvalue
    (:`0`
      (set `self.mass` 40000.0))
    (:`1`
      (set `self.mass` 80000.0))
    (:`2`
      (set `self.mass` 150000.0))
    (:`3`
      (set `self.mass` 500000.0))
    (:`4`
      (set `self.mass` 60000.0))
    (:`5`
      (set `self.mass` 55000.0))
    (:`6`
      (set `self.mass` 60000.0))
    (:`7`
      (set `self.mass` 85000.0))
    (:`8`
      (set `self.mass` 120000.0)))
  (`PrimitiveComponent.SetMassOverrideInKg` _destructible "None" (`self.mass`) true))