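; BP_Planet is a planet actor that pulls ships toward its center within a spherical gravity influence zone.
; A radius setting rescales the planet mesh and sizes the influence sphere as a multiple of that radius, at construction or through SetRadius.
; Ships derived from GEBaseShip register the planet as a velocity effector while overlapping the sphere.
; GetVelocityDeltaForPosition returns pull that falls off linearly from full gravity at the surface to zero at the sphere's edge.
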(event `GEPlanetInterface.SetRadius`
  (params (radius :type "Float (single-precision)"))
  (set `self.PlanetRedius` radius)
  (`self.SetRadiusF`))

(event `self.GravityInfluence.OnComponentBeginOverlap`
  (params (OverlappedComponent :type "PrimitiveComponent Object Reference") (OtherActor :type "Actor Object Reference") (OtherComp :type "PrimitiveComponent Object Reference") (OtherBodyIndex :type Integer) (bFromSweep :type Boolean) (SweepResult :type "HitResult Structure (by ref)"))
  ;[1 1 1] Add To Effector
  (bind _asgebase_ship (cast `GEBaseShip` OtherActor))
  (`GEBaseShip.AddVelocityEffector` _asgebase_ship self))

(event `self.GravityInfluence.OnComponentEndOverlap`
  (params (OverlappedComponent :type "PrimitiveComponent Object Reference") (OtherActor :type "Actor Object Reference") (OtherComp :type "PrimitiveComponent Object Reference") (OtherBodyIndex :type Integer))
  ;[1 1 1] Add To Effector
  (bind _asgebase_ship (cast `GEBaseShip` OtherActor))
  (`GEBaseShip.removeVelocityEffector` _asgebase_ship self))

(fn `GetVelocityDeltaForPosition`
  (params (Position :type "Vector Structure"))
  (returns (ReturnValue :type "Vector Structure"))
  (bind _planetredius (`self.PlanetRedius`))
  (bind _returnvalue (- (`self.K2_GetActorLocation`) Position))
  (bind _returnvalue_2 (`KismetMathLibrary.VSize` _returnvalue))
  (return (* (* (/ _returnvalue _returnvalue_2) (`self.Gravity`)) (- 1.0 (/ (- _returnvalue_2 _planetredius) (- (`self.GravityInfluenceExtent`) _planetredius))))))

(fn `SetRadiusF`
  (`SceneComponent.SetWorldScale3D` (`self.Planet`) (`KismetMathLibrary.Conv_DoubleToVector` (/ (`self.PlanetRedius`) (`.SphereRadius` (`KismetSystemLibrary.GetComponentBounds` (`self.Planet`))))))
  (bind _output_get (set `self.GravityInfluenceExtent` (* (`self.PlanetRedius`) (`self.GravityInflunceScale`))))
  (`SphereComponent.SetSphereRadius` (`self.GravityInfluence`) _output_get false))

(fn `UserConstructionScript`
  (`self.SetRadiusF`))