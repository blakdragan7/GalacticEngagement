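; Configurable static mesh actor that swaps in a chosen mesh and tints its materials at construction time.
; The construction script assigns a separate material to each of the first three slots.
; It then applies shared primary and secondary colours, roughness and metallic multipliers to every slot.
; Each parameter write makes its own CreateDynamicMaterialInstance call with MaterialOverride as the source, rather than reusing one instance per slot.
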(fn `UserConstructionScript`
  ;[1 1 1] Base mesh
  (`StaticMeshComponent.SetStaticMesh` (`self.Static_Mesh`) (`self.Replace Static Mesh`))
  (`|ExecutionSequence`
    (:`then_0`
      ;[1 1 1] Change colour, roughness, and metallic for material 1
      (`PrimitiveComponent.SetMaterial` (`self.Static_Mesh`) 0 (`self.New Material`))
      (`|ExecutionSequence`
        (:`then_0`
          (bind _returnvalue (`PrimitiveComponent.CreateDynamicMaterialInstance` (`self.Static_Mesh`) 0 (`self.Material Override`)))
          (`MaterialInstanceDynamic.SetVectorParameterValue` _returnvalue "Color" (`self.MaskColour`))
          (bind _returnvalue_2 (`PrimitiveComponent.CreateDynamicMaterialInstance` (`self.Static_Mesh`) 0 (`self.Material Override`)))
          (`MaterialInstanceDynamic.SetVectorParameterValue` _returnvalue_2 "Second Color" (`self.MaskColour 2`)))
        (:`then_1`
          (bind _returnvalue_3 (`PrimitiveComponent.CreateDynamicMaterialInstance` (`self.Static_Mesh`) 0 (`self.Material Override`)))
          (`MaterialInstanceDynamic.SetVectorParameterValue` _returnvalue_3 "Roughness Multiplier" (`self.Roughness Value`)))
        (:`then_2`
          (bind _returnvalue_4 (`PrimitiveComponent.CreateDynamicMaterialInstance` (`self.Static_Mesh`) 0 (`self.Material Override`)))
          (`MaterialInstanceDynamic.SetVectorParameterValue` _returnvalue_4 "Metallic Multiplier" (`self.Metallic Value`)))))
    (:`then_1`
      ;[1 1 1] Change colour, roughness, and metallic for material 2
      (`PrimitiveComponent.SetMaterial` (`self.Static_Mesh`) 1 (`self.New Material 2`))
      (`|ExecutionSequence`
        (:`then_0`
          (bind _returnvalue_5 (`PrimitiveComponent.CreateDynamicMaterialInstance` (`self.Static_Mesh`) 1 (`self.Material Override`)))
          (`MaterialInstanceDynamic.SetVectorParameterValue` _returnvalue_5 "Color" (`self.MaskColour`))
          (bind _returnvalue_6 (`PrimitiveComponent.CreateDynamicMaterialInstance` (`self.Static_Mesh`) 1 (`self.Material Override`)))
          (`MaterialInstanceDynamic.SetVectorParameterValue` _returnvalue_6 "Second Color" (`self.MaskColour 2`)))
        (:`then_1`
          (bind _returnvalue_7 (`PrimitiveComponent.CreateDynamicMaterialInstance` (`self.Static_Mesh`) 1 (`self.Material Override`)))
          (`MaterialInstanceDynamic.SetVectorParameterValue` _returnvalue_7 "Roughness Multiplier" (`self.Roughness Value`)))
        (:`then_2`
          (bind _returnvalue_8 (`PrimitiveComponent.CreateDynamicMaterialInstance` (`self.Static_Mesh`) 1 (`self.Material Override`)))
          (`MaterialInstanceDynamic.SetVectorParameterValue` _returnvalue_8 "Metallic Multiplier" (`self.Metallic Value`)))))
    (:`then_2`
      ;[1 1 1] Change colour, roughness, and metallic for material 3
      (`PrimitiveComponent.SetMaterial` (`self.Static_Mesh`) 2 (`self.New Material 3`))
      (`|ExecutionSequence`
        (:`then_0`
          (bind _returnvalue_9 (`PrimitiveComponent.CreateDynamicMaterialInstance` (`self.Static_Mesh`) 2 (`self.Material Override`)))
          (`MaterialInstanceDynamic.SetVectorParameterValue` _returnvalue_9 "Color" (`self.MaskColour`))
          (bind _returnvalue_10 (`PrimitiveComponent.CreateDynamicMaterialInstance` (`self.Static_Mesh`) 2 (`self.Material Override`)))
          (`MaterialInstanceDynamic.SetVectorParameterValue` _returnvalue_10 "Second Color" (`self.MaskColour 2`)))
        (:`then_1`
          (bind _returnvalue_11 (`PrimitiveComponent.CreateDynamicMaterialInstance` (`self.Static_Mesh`) 2 (`self.Material Override`)))
          (`MaterialInstanceDynamic.SetVectorParameterValue` _returnvalue_11 "Roughness Multiplier" (`self.Roughness Value`)))
        (:`then_2`
          (bind _returnvalue_12 (`PrimitiveComponent.CreateDynamicMaterialInstance` (`self.Static_Mesh`) 2 (`self.Material Override`)))
          (`MaterialInstanceDynamic.SetVectorParameterValue` _returnvalue_12 "Metallic Multiplier" (`self.Metallic Value`)))))))